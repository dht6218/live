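; BP_NPC is a talkable NPC actor that shows a random dialogue when the player presses F nearby.
; Box overlap with the player reveals a Plane and opens a Gate on the F input, and leaving reverses both.
; A FlipFlop alternates between opening WBP_NPC_Dialogue with a random NPCTalkPool entry and removing it, switching input mode and the player's Canmove flag each time.
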(event OnComponentBeginOverlap(Box)
  (params (OverlappedComponent :type Primitive%20Component%20Object%20Reference) (OtherActor :type Actor%20Object%20Reference) (OtherComp :type Primitive%20Component%20Object%20Reference) (OtherBodyIndex :type Integer) (bFromSweep :type Boolean) (SweepResult :type Hit%20Result%20Structure%20%28by%20ref%29))
  (bind _returnvalue (Game|GetPlayerController 0))
  (bind _npc_talkpool (Variables|Default|GetNPC_TalkPool))
  (bind _asplayer (Utilities|Casting|CastToplayer OtherActor))
  (Development|SetHiddeninGame (Variables|Default|GetPlane) false false)
  (Utilities|FlowControl|Gate true) ; enters at Open
)

(event OnComponentEndOverlap(Box)
  (params (OverlappedComponent :type Primitive%20Component%20Object%20Reference) (OtherActor :type Actor%20Object%20Reference) (OtherComp :type Primitive%20Component%20Object%20Reference) (OtherBodyIndex :type Integer))
  (bind _returnvalue (Game|GetPlayerController 0))
  (bind _npc_talkpool (Variables|Default|GetNPC_TalkPool))
  (Utilities|Casting|CastToplayer OtherActor)
  (Development|SetHiddeninGame (Variables|Default|GetPlane) true false)
  (Utilities|FlowControl|Gate true) ; enters at Close
)

(event EventBeginPlay
  (Input|EnableInput (Game|GetPlayerController 0))
  (Development|SetHiddeninGame (Variables|Default|GetPlane) true false))

(event Collision|EventActorBeginOverlap
  (params (OtherActor :type Actor%20Object%20Reference)))

(event EventTick
  (params (DeltaSeconds :type Float%20%28single-precision%29)))

(event Input|KeyboardEvents|F
  (params (Key :type Key%20Structure :default "None"))
  (bind _returnvalue (Game|GetPlayerController 0))
  (bind _npc_talkpool (Variables|Default|GetNPC_TalkPool))
  (:Pressed
    (Utilities|FlowControl|Gate true
      (:Exit
        (Utilities|FlowControl|FlipFlop
          (:A
            (bind _returnvalue_2 (UserInterface|CreateWidget "/Game/BP/fortext/WBP_NPC_Dialogue.WBP_NPC_Dialogue_C" 0 (Utilities|Array|Get(acopy) _npc_talkpool (Math|Random|RandomIntegerinRange 0 (Utilities|Array|LastIndex _npc_talkpool)))))
            (UserInterface|Viewport|AddtoViewport _returnvalue_2 0)
            (Input|SetInputModeGameandUI _returnvalue 0 "DoNotLock" true false)
            (Variables|/Game/BP/forplayer/player.player_C|Setcanmove (stale OnComponentBeginOverlap(Box) _asplayer) false))
          (:B
            (Input|SetInputModeGameOnly _returnvalue true)
            (Variables|/Game/BP/forplayer/player.player_C|Setcanmove (stale OnComponentBeginOverlap(Box) _asplayer) true)
            (Widget|RemovefromParent _returnvalue_2)))))))

(fn ConstructionScript)